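; BP_MyCharacter is a player character for what appears to be a two-team tag game.
; On BeginPlay it restricts player 0 to UI-only input for 30 seconds, then switches to game-only input.
; Left Shift launches the character forward as a dash, overriding its current velocity.
; Overlapping a character with a different IsBlueTeam value prints a Turkish message declaring the red team the winner, regardless of which side triggered it.
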(event Collision|EventActorBeginOverlap
  (params (OtherActor :type Actor%20Object%20Reference))
  (bind _asbp_my_character (Utilities|Casting|CastToBP_MyCharacter OtherActor))
  (if (!= (Variables|BP_MyCharacter_C|GetIsBlueTeam _asbp_my_character) (Variables|Default|GetIsBlueTeam))
    (Development|PrintString "Sure dolmadan yakalandi! Kirmizi Takim Kazandi!")))

(event EventTick
  (params (DeltaSeconds :type Float%20%28single-precision%29)))

(event EventBeginPlay
  (bind _returnvalue (Game|GetPlayerController 0))
  (Input|SetInputModeUIOnly _returnvalue 0 "DoNotLock" false)
  (Utilities|FlowControl|Delay 3e+01)
  (Input|SetInputModeGameOnly _returnvalue false))

(event Input|KeyboardEvents|LeftShift
  (params (Key :type Key%20Structure :default "None"))
  (:Pressed
    (Character|LaunchCharacter (* (Transformation|GetActorForwardVector) 2e+03) true true)))

(fn ConstructionScript)