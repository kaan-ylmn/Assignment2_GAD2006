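; BP_MyGameMode is a game mode that splits players into blue and red teams and declares blue the winner after 30 seconds.
; PostLogin alternates each joining player's BP_MyCharacter team flag through a toggled boolean.
; A one-shot timer from BeginPlay prints the blue win message, then swaps the locations of the last blue and last red characters found among all BP_MyCharacter actors.
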(event Custom|MaviTakimKazandi
  (Development|PrintString "30 Saniye Doldu - Mavi Takim Kazandi!")
  (bind _outactors (Actor|GetAllActorsOfClass "/Game/BP_MyCharacter.BP_MyCharacter_C"))
  ;[1 1 1] Looping through all players. Picked the last blue and red player to swap their locations.
  (for _array_element _outactors
    (if (Variables|/Game/BP_MyCharacter.BP_MyCharacter_C|GetIsBlueTeam _array_element)
      (Variables|Default|SetKazananMavi _array_element)
      (else
        (Variables|Default|SetSecilenKirmizi _array_element))))
  (Variables|Default|SetMaviEskiKonum (Transformation|GetActorLocation (Variables|Default|GetKazananMavi)))
  (Transformation|SetActorLocation (Variables|Default|GetKazananMavi) (Transformation|GetActorLocation (Variables|Default|GetSecilenKirmizi)) false false)
  (Transformation|SetActorLocation (Variables|Default|GetSecilenKirmizi) (Variables|Default|GetMaviEskiKonum) false false))

(event EventBeginPlay
  (Utilities|Time|SetTimerbyEvent (delegate Custom|MaviTakimKazandi) 3e+01))

(event EventTick
  (params (DeltaSeconds :type Float%20%28single-precision%29)))

(event EventPostLogin
  (params (NewPlayer :type Player%20Controller%20Object%20Reference))
  (bind _asbp_my_character (Utilities|Casting|CastToBP_MyCharacter (Pawn|GetControlledPawn NewPlayer)))
  (Variables|/Game/BP_MyCharacter.BP_MyCharacter_C|SetIsBlueTeam _asbp_my_character (Variables|Default|GetSiradakiMaviMi))
  (Variables|Default|SetSiradakiMaviMi (not (Variables|Default|GetSiradakiMaviMi))))

(fn ConstructionScript)